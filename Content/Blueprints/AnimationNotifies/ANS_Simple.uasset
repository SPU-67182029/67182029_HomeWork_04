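; ANS_Simple is an animation notify state that prints debug messages over its active window on an animation.
; Begin, tick and end each cast the mesh owner to BP_ThirdPersonCharacter and print the phase with the character's display name.
; The tick message also shows the frame delta time.
; Each handler returns true on a successful cast and false otherwise.
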(fn `Received_NotifyBegin`
  (params (MeshComp :type "SkeletalMeshComponent Object Reference") (Animation :type "AnimSequenceBase Object Reference") (TotalDuration :type "Float (single-precision)") (EventReference :type "AnimNotifyEventReference Structure (by ref)"))
  (returns (ReturnValue :type Boolean))
  (bind _asbp_third_person_character (cast `/Game/Blueprints/Characters/Players/BP_ThirdPersonCharacter` (`ActorComponent.GetOwner` MeshComp))
    (:`then`
      (`KismetSystemLibrary.PrintString` null (`KismetTextLibrary.Conv_TextToString` (`|FormatText` "ANS_Simple Begin : {c}" (`KismetSystemLibrary.GetDisplayName` _asbp_third_person_character))))
      (return true))
    (:`CastFailed`
      (return false))))

(fn `Received_NotifyEnd`
  (params (MeshComp :type "SkeletalMeshComponent Object Reference") (Animation :type "AnimSequenceBase Object Reference") (EventReference :type "AnimNotifyEventReference Structure (by ref)"))
  (returns (ReturnValue :type Boolean))
  (bind _asbp_third_person_character (cast `/Game/Blueprints/Characters/Players/BP_ThirdPersonCharacter` (`ActorComponent.GetOwner` MeshComp))
    (:`then`
      (`KismetSystemLibrary.PrintString` null (`KismetTextLibrary.Conv_TextToString` (`|FormatText` "ANS_Simple End : {c}" (`KismetSystemLibrary.GetDisplayName` _asbp_third_person_character))))
      (return true))
    (:`CastFailed`
      (return false))))

(fn `Received_NotifyTick`
  (params (MeshComp :type "SkeletalMeshComponent Object Reference") (Animation :type "AnimSequenceBase Object Reference") (FrameDeltaTime :type "Float (single-precision)") (EventReference :type "AnimNotifyEventReference Structure (by ref)"))
  (returns (ReturnValue :type Boolean))
  (bind _asbp_third_person_character (cast `/Game/Blueprints/Characters/Players/BP_ThirdPersonCharacter` (`ActorComponent.GetOwner` MeshComp))
    (:`then`
      (`KismetSystemLibrary.PrintString` null (`KismetTextLibrary.Conv_TextToString` (`|FormatText` "ANS_Simple Tick : {C} [{Duration}]" (`KismetSystemLibrary.GetDisplayName` _asbp_third_person_character) FrameDeltaTime)))
      (return true))
    (:`CastFailed`
      (return false))))